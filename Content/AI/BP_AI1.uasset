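; Sword-wielding AI enemy character that fights with montage combos and can be stealth-assassinated from behind.
; Attack, apparently behavior-tree driven, starts index-based combos with buffered continuation; timer-looped blade traces and a separate sphere trace damage "Damagable"-tagged actors.
; Incoming damage triggers hit reactions and knockback, reduces health via BPCPlayerStats and ragdolls on death.
; A camera-facing prompt appears when the player is near; StealthBackAssasin plays the victim montage, ragdolls and returns attacker alignment.
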(event `self.ReceiveBeginPlay`
  (bind _aswp_dummy_hp (cast `/Game/UI/WP_Dummy_HP` (`WidgetComponent.GetWidget` (`self.HPBarDummy`))))
  (set `self.HPBarUI` _aswp_dummy_hp))

(event `self.ReceiveTick`
  (params (DeltaSeconds :type "Float (single-precision)"))
  (`SceneComponent.K2_SetWorldRotation` (`self.Assanitate Widget`) (`KismetMathLibrary.FindLookAtRotation` (`SceneComponent.K2_GetComponentLocation` (`self.Assanitate Widget`)) (`SceneComponent.K2_GetComponentLocation` (`PlayerCameraManager.TransformComponent` (`GameplayStatics.GetPlayerCameraManager` 0)))) false false)
  (`SceneComponent.K2_SetWorldRotation` (`self.HPBarDummy`) (`KismetMathLibrary.FindLookAtRotation` (`SceneComponent.K2_GetComponentLocation` (`self.Assanitate Widget`)) (`SceneComponent.K2_GetComponentLocation` (`PlayerCameraManager.TransformComponent` (`GameplayStatics.GetPlayerCameraManager` 0)))) false false))

(event `Ragdol,`
  (`|ExecutionSequence`
    (:`then_0`
      (`KismetSystemLibrary.Delay` 2.5)
      (`PrimitiveComponent.SetSimulatePhysics` (`self.Mesh`) true))
    (:`then_1`
      (`KismetSystemLibrary.Delay` 1.7)
      (`GameplayStatics.PlaySoundAtLocation` "/Game/Audio/Hit/scDEATH.scDEATH" (`self.K2_GetActorLocation`) (struct) 1.0 1.0 0.0 "/Game/Audio/SA_Character.SA_Character" null null null))))

(event `self.AssasinationRadious.OnComponentBeginOverlap`
  (params (OverlappedComponent :type "PrimitiveComponent Object Reference") (OtherActor :type "Actor Object Reference") (OtherComp :type "PrimitiveComponent Object Reference") (OtherBodyIndex :type Integer) (bFromSweep :type Boolean) (SweepResult :type "HitResult Structure (by ref)"))
  (cast `/Game/ThirdPerson/Blueprints/BP_ThirdPersonCharacter` OtherActor)
  (`SceneComponent.SetVisibility` (`self.Assanitate Widget`) true false))

(event `self.AssasinationRadious.OnComponentEndOverlap`
  (params (OverlappedComponent :type "PrimitiveComponent Object Reference") (OtherActor :type "Actor Object Reference") (OtherComp :type "PrimitiveComponent Object Reference") (OtherBodyIndex :type Integer))
  (cast `/Game/ThirdPerson/Blueprints/BP_ThirdPersonCharacter` OtherActor)
  (`SceneComponent.SetVisibility` (`self.Assanitate Widget`) false false))

(event `self.ReceiveAnyDamage`
  (params (Damage :type "Float (single-precision)") (DamageType :type "DamageType Object Reference") (InstigatedBy :type "Controller Object Reference") (DamageCauser :type "Actor Object Reference"))
  (`self.PlayAnimMontage` (`|GetArrayItem` (`self.hitAnims`) (`KismetMathLibrary.RandomIntegerInRange` 0 (- (`KismetArrayLibrary.Array_Length` (`self.hitAnims`)) 1))))
  (bind _asbp_third_person_character (cast `/Game/ThirdPerson/Blueprints/BP_ThirdPersonCharacter` (`GameplayStatics.GetPlayerCharacter` 0)))
  (`self.LaunchCharacter` (* (`KismetMathLibrary.GetForwardVector` (`self.K2_GetActorRotation` _asbp_third_person_character)) 700.0))
  (`GameplayStatics.PlaySoundAtLocation` "/Game/Audio/Hit/416839__tonsil5__grunt1-death-pain.416839__tonsil5__grunt1-death-pain" (`self.K2_GetActorLocation`) (struct) (`KismetMathLibrary.RandomFloatInRange` -1.5 1.5) 1.0 0.0 "/Game/Audio/SA_Character.SA_Character" null null null)
  (bind _isplayerdead (`/Game/Blueprints/BPC_PlayerStats.decreaseHP` (`self.BPC_PlayerStats`) Damage))
  (if _isplayerdead
    (`PrimitiveComponent.SetCollisionObjectType` (`self.Mesh`) "ECC_PhysicsBody")
    (`PrimitiveComponent.SetSimulatePhysics` (`self.Mesh`) true)
    (`GameplayStatics.PlaySoundAtLocation` "/Game/Audio/Hit/scDEATH.scDEATH" (`self.K2_GetActorLocation`) (struct) 1.0 1.0 0.0 "/Game/Audio/SA_Character.SA_Character" null null null)
    (`SceneComponent.SetVisibility` (`self.HPBarDummy`) false false)))

(event `SwordAttackComboFromBT`
  ;[1 1 1] Attack and input
  (if (`self.canAttack?`)
    (`self.SwordAttack`)))

(event `Attack1`
  ;[1 1 1] Attack1
  (`/Engine/EditorBlueprintResources/StandardMacros.DoOnce` false :!label _label
    (:`Completed`
      (`KismetSystemLibrary.Delay` 0.1)
      (`|PlayMontage` (`self.Mesh`) "/Game/Characters/RPG_Character/Animation/SwordAttack/Attack1_Montage.Attack1_Montage"
        (:`then`
          (set `self.attackIndex` 1)
          (goto _label :!via `Reset`))))))

(event `SwordAttack`
  ;[1 1 1] Sword attack
  (if (`self.isAttacking?`)
    (set `self.saveAttack` true)
    (else
      (set `self.isAttacking?` true)
      (switch `int` (`self.attackIndex`) :!label _label_2
        (:`0`
          (`self.Attack1`))
        (:`1`
          (`self.attack2`))
        (:`2`
          (`self.attack4`))))))

(event `attack2`
  ;[1 1 1] Attack2
  (`/Engine/EditorBlueprintResources/StandardMacros.DoOnce` false :!label _label_3
    (:`Completed`
      (`KismetSystemLibrary.Delay` 0.1)
      (`|PlayMontage` (`self.Mesh`) "/Game/Characters/RPG_Character/Animation/SwordAttack/Attack2_Montage.Attack2_Montage"
        (:`then`
          (set `self.attackIndex` 2)
          (goto _label_3 :!via `Reset`))))))

(event `SwordAttackCombo`
  ;[1 1 1] Combo continue
  (if (`self.saveAttack`)
    (set `self.saveAttack` false)
    (goto _label_2)
    (else
      (`self.StopCombo`))))

(event `attack3`
  ;[1 1 1] Attack3
  (`/Engine/EditorBlueprintResources/StandardMacros.DoOnce` false :!label _label_4
    (:`Completed`
      (`KismetSystemLibrary.Delay` 0.1)
      (`|PlayMontage` (`self.Mesh`) "/Game/Characters/RPG_Character/Animation/SwordAttack/Kick_Montage.Kick_Montage"
        (:`then`
          (set `self.attackIndex` 3)
          (goto _label_4 :!via `Reset`))))))

(event `StopCombo`
  ;[1 1 1] Stop combo
  (set `self.isAttacking?` false)
  (set `self.attackIndex` 0))

(event `attack4`
  ;[1 1 1] Attack4
  (`/Engine/EditorBlueprintResources/StandardMacros.DoOnce` false :!label _label_5
    (:`Completed`
      (`KismetSystemLibrary.Delay` 0.1)
      (`|PlayMontage` (`self.Mesh`) "/Game/Characters/RPG_Character/Animation/SwordAttack/Attack3_Montage.Attack3_Montage"
        (:`then`
          (set `self.attackIndex` 4)
          (goto _label_5 :!via `Reset`))))))

(event `swordTraceStart`
  ;[1 1 1] SwordTrace
  (bind _returnvalue (`KismetSystemLibrary.K2_SetTimerDelegate` (delegate `swordTraceLoop`) 0.01 true))
  (set `self.SwordTraceLoopvar` _returnvalue))

(event `swordTraceLoop`
  ;[1 1 1] SwordTrace
  (bind (_outhit _returnvalue) (`KismetSystemLibrary.SphereTraceSingle` :`Start` (`SceneComponent.K2_GetComponentLocation` (`self.swordTopPoint`)) :`End` (`SceneComponent.K2_GetComponentLocation` (`self.swordBottomPoint`)) :`Radius` 12.0 :`TraceChannel` "TraceTypeQuery1" :`DrawDebugType` "ForDuration" :`DrawTime` 3.0))
  (if _returnvalue
    (bind (_bblockinghit _binitialoverlap _time _distance _location _impactpoint _normal _impactnormal _physmat _hitactor) (`GameplayStatics.BreakHitResult` _outhit))
    (if (`self.ActorHasTag` _hitactor "Damagable")
      (`/Engine/EditorBlueprintResources/StandardMacros.DoOnce` false :!label _label_6
        (:`Completed`
          (`GameplayStatics.ApplyDamage` _hitactor 10.0)
          (`GameplayStatics.PlayWorldCameraShake` "/Game/Blueprints/BP_Hit_Camera_Shake.BP_Hit_Camera_Shake_C" _location 0.0 2000.0)
          (`self.playSwordHitSounds`)
          (`GameplayStatics.SpawnEmitterAtLocation` "/Game/Realistic_Starter_VFX_Pack_Vol2/Particles/Blood/P_Blood_Splat_Cone.P_Blood_Splat_Cone" _location (`KismetMathLibrary.MakeRotFromXY` _normal _normal) (0.4 0.4 0.4) true "AutoRelease")
          (`KismetSystemLibrary.Delay` 0.5)
          (goto _label_6 :!via `Reset`))))))

(event `swordStopTrace`
  ;[1 1 1] SwordTrace
  (`KismetSystemLibrary.K2_ClearAndInvalidateTimerHandle` (`self.SwordTraceLoopvar`)))

(event `playSwordHitSounds`
  ;[1 1 1] playSwordHitsounds
  (`GameplayStatics.PlaySoundAtLocation` "/Game/Audio/SwordHits/Ms_Sword_HIT.Ms_Sword_HIT" (`self.K2_GetActorLocation` (`self.GetOwner`)) (struct) 1.0 1.0 0.0 null null null null))

(event `SphereTrace`
  (bind _returnvalue (`SceneComponent.K2_GetComponentLocation` (`self.SphereTracePOS`)))
  ;[1 1 1] SphereTrace(For kick and stab)
  (bind (_outhit _returnvalue_2) (`KismetSystemLibrary.SphereTraceSingle` :`Start` _returnvalue :`End` _returnvalue :`Radius` 25.0 :`TraceChannel` "TraceTypeQuery1" :`DrawDebugType` "ForDuration"))
  (if _returnvalue_2
    (bind (_bblockinghit _binitialoverlap _time _distance _location _impactpoint _normal _impactnormal _physmat _hitactor) (`GameplayStatics.BreakHitResult` _outhit))
    (if (`self.ActorHasTag` _hitactor "Damagable")
      (`GameplayStatics.ApplyDamage` _hitactor 10.0)
      (`GameplayStatics.PlayWorldCameraShake` "/Game/Blueprints/BP_Hit_Camera_Shake.BP_Hit_Camera_Shake_C" _location 0.0 2000.0)
      (`self.playSwordHitSounds`)
      (`GameplayStatics.SpawnEmitterAtLocation` "/Game/Realistic_Starter_VFX_Pack_Vol2/Particles/Blood/P_Blood_Splat_Cone.P_Blood_Splat_Cone" _location (`KismetMathLibrary.MakeRotFromXY` _normal _normal) (0.4 0.4 0.4) true "AutoRelease"))))

(fn `Attack`
  (returns (animationDuration :type "Float (double-precision)"))
  (`self.SwordAttackComboFromBT`)
  (return 0.4))

(fn `StealthBackAssasin`
  (returns (ReferenceLocation :type "Vector Structure") (AssasinRotation :type "Rotator Structure"))
  (`self.PlayAnimMontage` "/Game/Characters/RPG_Character/Animation/Assasination/Paired_Knife_Stealth_KidneyAndNeck_Vic_Montage.Paired_Knife_Stealth_KidneyAndNeck_Vic_Montage")
  (`self.Ragdol,`)
  (`SceneComponent.SetVisibility` (`self.Assanitate Widget`) false false)
  (return (`SceneComponent.K2_GetComponentLocation` (`self.AssasinReference`)) (`self.K2_GetActorRotation`)))

(fn `UserConstructionScript`)