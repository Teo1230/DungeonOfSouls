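; Player stats component for BP_ThirdPersonCharacter that tracks HP, mana, XP and level.
; On BeginPlay it waits a tick, caches the owning character and fills its HUD widget, which each stat function then updates directly.
; Decrease functions return whether the stat is depleted, and increase functions cap at the maximum.
; Reaching max XP triggers a level-up that raises the threshold, discards leftover XP and plays sounds.
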(event `self.ReceiveBeginPlay`
  (bind _hudwidget (`/Game/ThirdPerson/Blueprints/BP_ThirdPersonCharacter.HudWidget` (`self.character`)))
  (bind _hudwidget_2 (`/Game/ThirdPerson/Blueprints/BP_ThirdPersonCharacter.HudWidget` (`self.character`)))
  (`KismetSystemLibrary.DelayUntilNextTick`)
  (bind _asbp_third_person_character (cast `/Game/ThirdPerson/Blueprints/BP_ThirdPersonCharacter` (`self.GetOwner`)))
  (set `self.character` _asbp_third_person_character)
  ;[1 1 1] da err
  (`ProgressBar.SetPercent` (`/Game/UI/BLP_HUD.HP` _hudwidget_2) (/ (`self.currentHP`) (`self.maxHP`)))
  (`TextBlock.SetText` (`/Game/UI/BLP_HUD.HPtext` _hudwidget_2) (`KismetTextLibrary.Conv_DoubleToText` (`self.currentHP`) "HalfToEven"))
  (`ProgressBar.SetPercent` (`/Game/UI/BLP_HUD.MN` _hudwidget) (/ (`self.currentMN`) (`self.maxMN`)))
  (`TextBlock.SetText` (`/Game/UI/BLP_HUD.Manatext` _hudwidget) (`KismetTextLibrary.Conv_DoubleToText` (`self.currentMN`) "HalfToEven"))
  (`ProgressBar.SetPercent` (`/Game/UI/BLP_HUD.XPBAR` (`/Game/ThirdPerson/Blueprints/BP_ThirdPersonCharacter.HudWidget` (`self.character`))) (/ (`self.XP`) (`self.maxXP`)))
  (`TextBlock.SetText` (`/Game/UI/BLP_HUD.XPText` (`/Game/ThirdPerson/Blueprints/BP_ThirdPersonCharacter.HudWidget` (`self.character`))) (`|FormatText` "{CurrentXP} /{MAXXP}" (`self.XP`) (`self.maxXP`)))
  (`TextBlock.SetText` (`/Game/UI/BLP_HUD.LevelText` (`/Game/ThirdPerson/Blueprints/BP_ThirdPersonCharacter.HudWidget` (`self.character`))) (`KismetTextLibrary.Conv_IntToText` (`self.level`))))

(fn `decreaseHP`
  (params (damage :type "Float (double-precision)"))
  (returns (isPlayerDead :type Boolean))
  (bind _hudwidget (`/Game/ThirdPerson/Blueprints/BP_ThirdPersonCharacter.HudWidget` (`self.character`)))
  (if (not (<= (`self.currentHP`) 0.0))
    (bind _output_get (set `self.currentHP` (- (`self.currentHP`) damage)))
    (`ProgressBar.SetPercent` (`/Game/UI/BLP_HUD.HP` _hudwidget) (/ _output_get (`self.maxHP`)))
    (`TextBlock.SetText` (`/Game/UI/BLP_HUD.HPtext` _hudwidget) (`KismetTextLibrary.Conv_DoubleToText` (`self.currentHP`) "HalfToEven"))
    (if (<= (`self.currentHP`) 0.0)
      _
      (else
        (return false))))
  (return true))

(fn `decreaseMN`
  (params (MNdeplited :type "Float (double-precision)"))
  (returns (notMNLeft :type Boolean))
  (bind _hudwidget (`/Game/ThirdPerson/Blueprints/BP_ThirdPersonCharacter.HudWidget` (`self.character`)))
  (if (not (<= (`self.currentMN`) 0.0))
    (bind _output_get (set `self.currentMN` (- (`self.currentMN`) MNdeplited)))
    (`ProgressBar.SetPercent` (`/Game/UI/BLP_HUD.MN` _hudwidget) (/ _output_get (`self.maxMN`)))
    (`TextBlock.SetText` (`/Game/UI/BLP_HUD.Manatext` _hudwidget) (`KismetTextLibrary.Conv_DoubleToText` (`self.currentMN`) "HalfToEven"))
    (if (<= (`self.currentMN`) 0.0)
      _
      (else
        (return false))))
  (return true))

(fn `IncreaseHP`
  (params (addedHP :type "Float (double-precision)"))
  (bind _hudwidget (`/Game/ThirdPerson/Blueprints/BP_ThirdPersonCharacter.HudWidget` (`self.character`)))
  (set `self.currentHP` (+ (`self.currentHP`) addedHP))
  (if (> (`self.currentHP`) (`self.maxHP`))
    (set `self.currentHP` (`self.maxHP`)))
  (`ProgressBar.SetPercent` (`/Game/UI/BLP_HUD.HP` _hudwidget) (/ (`self.currentHP`) (`self.maxHP`)))
  (`TextBlock.SetText` (`/Game/UI/BLP_HUD.HPtext` _hudwidget) (`KismetTextLibrary.Conv_DoubleToText` (`self.currentHP`) "HalfToEven")))

(fn `IncreaseLEVEL`
  (params (AddedLevel :type Integer))
  (set `self.level` (+ (`self.level`) AddedLevel))
  (set `self.maxXP` (+ (`self.maxXP`) 50.0))
  (set `self.XP` 0.0)
  (`TextBlock.SetText` (`/Game/UI/BLP_HUD.LevelText` (`/Game/ThirdPerson/Blueprints/BP_ThirdPersonCharacter.HudWidget` (`self.character`))) (`KismetTextLibrary.Conv_IntToText` (`self.level`)))
  (`GameplayStatics.PlaySound2D` "/Game/Audio/UI/level1.level1" 1.0 1.0 0.0 null null)
  (`GameplayStatics.PlaySound2D` "/Game/Audio/UI/level2.level2" 1.0 1.0 0.0 null null))

(fn `increaseMaxHP`
  (params (HPincremention :type "Float (double-precision)"))
  (bind _hudwidget (`/Game/ThirdPerson/Blueprints/BP_ThirdPersonCharacter.HudWidget` (`self.character`)))
  (set `self.maxHP` (+ HPincremention (`self.maxHP`)))
  (`ProgressBar.SetPercent` (`/Game/UI/BLP_HUD.HP` _hudwidget) (/ (`self.currentHP`) (`self.maxHP`)))
  (`TextBlock.SetText` (`/Game/UI/BLP_HUD.HPtext` _hudwidget) (`KismetTextLibrary.Conv_DoubleToText` (`self.currentHP`) "HalfToEven")))

(fn `IncreaseMaxMN`
  (params (incrementMN :type "Float (double-precision)"))
  (bind _hudwidget (`/Game/ThirdPerson/Blueprints/BP_ThirdPersonCharacter.HudWidget` (`self.character`)))
  (set `self.maxMN` (+ (`self.maxMN`) incrementMN))
  (`ProgressBar.SetPercent` (`/Game/UI/BLP_HUD.MN` _hudwidget) (/ (`self.currentMN`) (`self.maxMN`)))
  (`TextBlock.SetText` (`/Game/UI/BLP_HUD.Manatext` _hudwidget) (`KismetTextLibrary.Conv_DoubleToText` (`self.currentMN`) "HalfToEven")))

(fn `IncreaseMN`
  (params (addedMN :type "Float (double-precision)"))
  (bind _hudwidget (`/Game/ThirdPerson/Blueprints/BP_ThirdPersonCharacter.HudWidget` (`self.character`)))
  (set `self.currentMN` (+ (`self.currentMN`) addedMN))
  (if (> (`self.currentMN`) (`self.maxMN`))
    (set `self.currentMN` (`self.maxMN`)))
  (`ProgressBar.SetPercent` (`/Game/UI/BLP_HUD.MN` _hudwidget) (/ (`self.currentMN`) (`self.maxMN`)))
  (`TextBlock.SetText` (`/Game/UI/BLP_HUD.Manatext` _hudwidget) (`KismetTextLibrary.Conv_DoubleToText` (`self.currentMN`) "HalfToEven")))

(fn `IncreaseXP`
  (params (AddedXP :type "Float (double-precision)"))
  (set `self.XP` (+ (`self.XP`) AddedXP))
  (if (>= (`self.XP`) (`self.maxXP`))
    (`self.IncreaseLEVEL` 1))
  (`ProgressBar.SetPercent` (`/Game/UI/BLP_HUD.XPBAR` (`/Game/ThirdPerson/Blueprints/BP_ThirdPersonCharacter.HudWidget` (`self.character`))) (/ (`self.XP`) (`self.maxXP`)))
  (`TextBlock.SetText` (`/Game/UI/BLP_HUD.XPText` (`/Game/ThirdPerson/Blueprints/BP_ThirdPersonCharacter.HudWidget` (`self.character`))) (`|FormatText` "{CurrentXP} /{MAXXP}" (`self.XP`) (`self.maxXP`))))