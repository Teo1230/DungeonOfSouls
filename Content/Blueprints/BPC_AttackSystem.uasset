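; Actor component that gives the third-person character a four-step sword and kick melee combo.
; Attack input, gated by CanAttack, starts a montage chosen by AttackIndex, or sets SaveAttack to buffer input during an attack.
; SwordAttackCombo consumes the buffered input to play the next step, otherwise StopCombo resets the chain.
; Each step uses a DoOnce guard and short delay before playing its montage and advancing the index.
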(event `self.ReceiveBeginPlay`
  (bind _asbp_third_person_character (cast `/Game/ThirdPerson/Blueprints/BP_ThirdPersonCharacter` (`self.GetOwner`)))
  (set `self.charachterMesh` (`Character.Mesh` _asbp_third_person_character)))

(event `InputAction|Atack`
  (params (Key :type "Key Structure"))
  ;[1 1 1] Attack and input
  (:`Pressed`
    (if (`self.canAttack?`)
      (`self.SwordAttack`))))

(event `Attack1`
  ;[1 1 1] Attack1
  (`/Engine/EditorBlueprintResources/StandardMacros.DoOnce` false :!label _label
    (:`Completed`
      (`KismetSystemLibrary.Delay` 0.1)
      (`|PlayMontage` (`self.charachterMesh`) "/Game/Characters/RPG_Character/Animation/SwordAttack/Attack1_Montage.Attack1_Montage"
        (:`then`
          (set `self.attackIndex` 1)
          (goto _label :!via `Reset`))))))

(event `SwordAttack`
  ;[1 1 1] Sword attack
  (if (`self.isAttacking?`)
    (set `self.saveAttack` true)
    (else
      (set `self.isAttacking?` true)
      (switch `int` (`self.attackIndex`) :!label _label_2
        (:`0`
          (`self.Attack1`))
        (:`1`
          (`self.attack2`))
        (:`2`
          (`self.attack3`))
        (:`3`
          (`self.attack4`))))))

(event `attack2`
  ;[1 1 1] Attack2
  (`/Engine/EditorBlueprintResources/StandardMacros.DoOnce` false :!label _label_3
    (:`Completed`
      (`KismetSystemLibrary.Delay` 0.1)
      (`|PlayMontage` (`self.charachterMesh`) "/Game/Characters/RPG_Character/Animation/SwordAttack/Attack2_Montage.Attack2_Montage"
        (:`then`
          (set `self.attackIndex` 2)
          (goto _label_3 :!via `Reset`))))))

(event `SwordAttackCombo`
  ;[1 1 1] Combo continue
  (if (`self.saveAttack`)
    (set `self.saveAttack` false)
    (goto _label_2)
    (else
      (`self.StopCombo`))))

(event `attack3`
  ;[1 1 1] Attack3
  (`/Engine/EditorBlueprintResources/StandardMacros.DoOnce` false :!label _label_4
    (:`Completed`
      (`KismetSystemLibrary.Delay` 0.1)
      (`|PlayMontage` (`self.charachterMesh`) "/Game/Characters/RPG_Character/Animation/SwordAttack/Kick_Montage.Kick_Montage"
        (:`then`
          (set `self.attackIndex` 3)
          (goto _label_4 :!via `Reset`))))))

(event `StopCombo`
  ;[1 1 1] Stop combo
  (set `self.isAttacking?` false)
  (set `self.attackIndex` 0))

(event `attack4`
  ;[1 1 1] Attack4
  (`/Engine/EditorBlueprintResources/StandardMacros.DoOnce` false :!label _label_5
    (:`Completed`
      (`KismetSystemLibrary.Delay` 0.1)
      (`|PlayMontage` (`self.charachterMesh`) "/Game/Characters/RPG_Character/Animation/SwordAttack/Attack3_Montage.Attack3_Montage"
        (:`then`
          (set `self.attackIndex` 4)
          (goto _label_5 :!via `Reset`))))))